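; BP_Spikes is a moving obstacle in a cat runner game that kills the cat character on contact.
; Each tick it scrolls along negative X at the game mode's GameSpeed, scaled by delta time, so the world moves past the player.
; Overlapping a BP_CatCharacter calls its Death function.
; A looping timer periodically destroys the actor once it moves past a fixed X limit behind the view.
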(event Collision|EventActorBeginOverlap
  (params (OtherActor :type Actor%20Object%20Reference))
  (bind _asbp_cat_character (Utilities|Casting|CastToBP_CatCharacter OtherActor))
  (Default|Death _asbp_cat_character))

(event EventTick
  (params (DeltaSeconds :type Float%20%28single-precision%29))
  (Transformation|AddActorWorldOffset (Math|Vector|MakeVector (* DeltaSeconds (Variables|/Game/Blueprints/BP_Cat_Runner_GameMode.BP_Cat_Runner_GameMode_C|GetGameSpeed (Variables|Default|GetGameMode)) -1.0) 0.0 0.0)))

(event EventBeginPlay
  (bind _asbp_cat_runner_game_mode (Utilities|Casting|CastToBP_Cat_Runner_GameMode (Game|GetGameMode)))
  (Variables|Default|SetGameMode _asbp_cat_runner_game_mode)
  (Utilities|Time|SetTimerbyFunctionName 0 "DestroyIfOutGameView" 1.0 true))

(fn ConstructionScript)

(fn DestroyifOutGameView
  (if (< (.x (Transformation|GetActorLocation)) -1.4e+03)
    (Actor|DestroyActor)))