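; Game mode for an endless cat runner that spawns spikes or saws at random intervals and tracks distance on the HUD.
; Tick periodically multiplies game speed up to a cap, scaling the cat's jump velocity and recomputing gravity to keep jump height constant.
; Game over shows restart UI, zeroes ground and background scroll speeds in a material parameter collection, and fades game speed toward zero from its initial value.
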(event Custom|SpawnRandomObstacle
  (if (not (Variables|Default|GetGameIsOver))
    (Game|SpawnActorfromClass (select (Math|Random|RandomBool) "/Game/Blueprints/BP_Spikes.BP_Spikes_C" "/Game/Blueprints/BP_Saw.BP_Saw_C") (Math|Transform|MakeTransform "1400.000000,0.000000,-400.000000") "Undefined" 0 0)
    (Utilities|Time|SetTimerbyEvent (delegate Custom|SpawnRandomObstacle) (Math|Random|RandomFloatinRange 0.6 1.0))))

(event Custom|GameOver
  (Variables|Default|SetGameIsOver true)
  (Default|ShowRestartButton (Variables|Default|GetGameHUD))
  (Variables|/Script/Engine.PlayerController|SetbShowMouseCursor (Game|GetPlayerController 0) true)
  ;[1 1 1] Comment
  (Rendering|Material|SetVectorParameterValue "/Game/MTC.MTC" "GroundSpeed" (Utilities|Struct|MakeLinearColor 0.0 0.0 0.0 0.0) :!class /Script/Engine.KismetMaterialLibrary)
  (Rendering|Material|SetVectorParameterValue "/Game/MTC.MTC" "BackgroundSpeed" (Utilities|Struct|MakeLinearColor 0.0 0.0 0.0 0.0) :!class /Script/Engine.KismetMaterialLibrary))

(event EventBeginPlay
  (Utilities|FlowControl|Sequence
    (:then_0
      ;[1 1 1] Init Speed Params to Fade on Death
      (Utilities|FlowControl|Sequence
        (:then_0
          (Utilities|FlowControl|DoOnce false
            (:Completed
              (bind _returnvalue (Rendering|Material|GetVectorParameterValue "/Game/MTC.MTC" "GroundSpeed" :!class /Script/Engine.KismetMaterialLibrary))
              (Variables|Default|SetGroundSpeedInit (.r _returnvalue))
              (bind _returnvalue_2 (Rendering|Material|GetVectorParameterValue "/Game/MTC.MTC" "BackgroundSpeed" :!class /Script/Engine.KismetMaterialLibrary))
              (Variables|Default|SetBackgroundSpeedInit (.r _returnvalue_2))
              (Variables|Default|SetGameSpeedInit (Variables|Default|GetGameSpeed)))))
        (:then_1
          (Variables|Default|SetSpeedFadeCurrentAlpha 0.0)
          (Rendering|Material|SetVectorParameterValue "/Game/MTC.MTC" "GroundSpeed" (Utilities|Struct|MakeLinearColor (Variables|Default|GetGroundSpeedInit) 0.0 0.0 1.0) :!class /Script/Engine.KismetMaterialLibrary)
          (Rendering|Material|SetVectorParameterValue "/Game/MTC.MTC" "BackgroundSpeed" (Utilities|Struct|MakeLinearColor (Variables|Default|GetBackgroundSpeedInit) 0.0 0.0 1.0) :!class /Script/Engine.KismetMaterialLibrary))))
    (:then_1
      ;[1 1 1] Get Character Ref
      (bind _asbp_cat_character (Utilities|Casting|CastToBP_CatCharacter (Game|GetPlayerCharacter 0)))
      (bind _output_get (Variables|Default|SetCharacter _asbp_cat_character))
      (Variables|Default|SetInitJumpHeightWithGravity (* (Class|CharacterMovementComponent|GetMaxJumpHeight (Variables|/Script/Engine.Character|GetCharacterMovement _output_get)) -9.8e+02 -2.0)))
    (:then_2
      (Variables|Default|SetGameIsOver false)
      (bind _returnvalue_3 (UserInterface|CreateWidget "/Game/Blueprints/MAIN_HUD.MAIN_HUD_C"))
      (bind _output_get_2 (Variables|Default|SetGameHUD _returnvalue_3))
      (UserInterface|Viewport|AddtoViewport _output_get_2 0)
      (Utilities|Time|SetTimerbyEvent (delegate Custom|SpawnRandomObstacle) (Math|Random|RandomFloatinRange 0.6 1.0)))))

(event EventTick
  (params (DeltaSeconds :type Float%20%28single-precision%29))
  (if (not (Variables|Default|GetGameIsOver))
    (bind _output_get (Variables|Default|SetTotalDistance (+ (* (Variables|Default|GetGameSpeed) DeltaSeconds) (Variables|Default|GetTotalDistance))))
    (Default|UpdateDistanceText (Variables|Default|GetGameHUD) (/ _output_get 1e+02))
    (CallFunction|SpeedUpGame DeltaSeconds)
    (elif (> (Variables|Default|GetGameSpeed) 0.0)
      (CallFunction|FadeGameSpeedonDeath DeltaSeconds))))

(fn ConstructionScript)

(fn FadeGameSpeedonDeath
  (params (DeltaTime :type Float%20%28single-precision%29))
  ;[1 1 1] Calc current speed fade  alpha
  (Variables|Default|SetSpeedFadeCurrentAlpha (+ (* DeltaTime (Variables|Default|GetSpeedFadeSec)) (Variables|Default|GetSpeedFadeCurrentAlpha)))
  (Variables|Default|SetGameSpeed (Math|Float|Lerp (Variables|Default|GetGameSpeedInit) 0.0 (Variables|Default|GetSpeedFadeCurrentAlpha))))

(fn SpeedUpGame
  (params (DeltaTime :type Float%20%28single-precision%29))
  (bind _character (Variables|Default|GetCharacter))
  (bind _character_2 (Variables|Default|GetCharacter))
  (bind _charactermovement (Variables|/Script/Engine.Character|GetCharacterMovement _character_2))
  (bind _charactermovement_2 (Variables|/Script/Engine.Character|GetCharacterMovement _character))
  ;[1 1 1] SpeedUp Delay
  (Variables|Default|SetSpeedUpDelayAccomulation (+ DeltaTime (Variables|Default|GetSpeedUpDelayAccomulation)))
  (if (>= (Variables|Default|GetSpeedUpDelayAccomulation) (Variables|Default|GetSpeedUpDelay))
    (Variables|Default|SetSpeedUpDelayAccomulation 0.0)
    ;[1 1 1] Speed Up Clamp
    (if (< (/ (Variables|Default|GetGameSpeed) (Variables|Default|GetGameSpeedInit)) (Variables|Default|GetSpeedUpClamp))
      (Utilities|FlowControl|Sequence
        (:then_0
          ;[1 1 1] Obstacle Speed
          (Variables|Default|SetGameSpeed (* (Variables|Default|GetGameSpeed) (Variables|Default|GetSpeedUpFactor))))
        (:then_1
          ;[1 1 1] Scale Cat Jump Velocity
          (Variables|/Script/Engine.CharacterMovementComponent|SetJumpZVelocity _charactermovement_2 (* (Variables|/Script/Engine.CharacterMovementComponent|GetJumpZVelocity _charactermovement_2) (Variables|Default|GetSpeedUpFactor))))
        (:then_2
          ;[1 1 1] Calc And Scale Cat Gravity
          (Variables|/Script/Engine.CharacterMovementComponent|SetGravityScale _charactermovement (/ (Math|Float|Square (Variables|/Script/Engine.CharacterMovementComponent|GetJumpZVelocity _charactermovement)) (Variables|Default|GetInitJumpHeightWithGravity))))))))