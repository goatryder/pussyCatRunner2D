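; BP_Saw is a spinning saw obstacle in a cat runner game that kills BP_CatCharacter on overlap.
; Each tick it moves along negative X at the game mode's GameSpeed and spins its Paper2D sprite by RotationSpeed.
; A looping timer destroys it once it passes a fixed X limit out of view.
; When the game is over, the spin eases from its initial speed to zero through an accumulated lerp alpha.
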(event Collision|EventActorBeginOverlap
  (params (OtherActor :type Actor%20Object%20Reference))
  (bind _asbp_cat_character (Utilities|Casting|CastToBP_CatCharacter OtherActor))
  (Default|Death _asbp_cat_character))

(event EventTick
  (params (DeltaSeconds :type Float%20%28single-precision%29))
  (Transformation|AddActorWorldOffset (Math|Vector|MakeVector (* (Variables|/Game/Blueprints/BP_Cat_Runner_GameMode.BP_Cat_Runner_GameMode_C|GetGameSpeed (Variables|Default|GetGameMode)) -1.0 DeltaSeconds) 0.0 0.0))
  (Transformation|AddLocalRotation (Variables|Default|GetPaperSprite) (Math|Rotator|MakeRotator 0.0 (* (Variables|Default|GetRotationSpeed) DeltaSeconds) 0.0) false false)
  (if (Variables|/Game/Blueprints/BP_Cat_Runner_GameMode.BP_Cat_Runner_GameMode_C|GetGameIsOver (Variables|Default|GetGameMode))
    (CallFunction|RotationFadeonDeath DeltaSeconds)))

(event EventBeginPlay
  (Variables|Default|SetInitRotationSpeed (Variables|Default|GetRotationSpeed))
  (bind _asbp_cat_runner_game_mode (Utilities|Casting|CastToBP_Cat_Runner_GameMode (Game|GetGameMode)))
  (Variables|Default|SetGameMode _asbp_cat_runner_game_mode)
  (Utilities|Time|SetTimerbyFunctionName 0 "DestroyIfOutGameView" 1.0 true))

(fn ConstructionScript)

(fn DestroyifOutGameView
  (if (< (.x (Transformation|GetActorLocation)) -1.4e+03)
    (Actor|DestroyActor)))

(fn RotationFadeonDeath
  (params (DeltaSeconds :type Float%20%28single-precision%29))
  (if (> (Variables|Default|GetRotationSpeed) 0.0)
    ;[1 1 1] Calc current rotation speed fade  alpha
    (Variables|Default|SetRotationSpeedFadeAlpha (+ (* (Variables|Default|GetRotationSpeedFadeSec) DeltaSeconds) (Variables|Default|GetRotationSpeedFadeAlpha)))
    (Variables|Default|SetRotationSpeed (Math|Float|Lerp (Variables|Default|GetInitRotationSpeed) 0.0 (Variables|Default|GetRotationSpeedFadeAlpha)))))